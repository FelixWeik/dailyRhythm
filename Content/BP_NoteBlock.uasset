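; BP_NoteBlock is a colored note actor, apparently for a rhythm-style game, that travels in a straight line and removes itself.
; Its construction script tints the Cube through a dynamic material instance using NoteColor.
; Tick slides the Cube along local negative X at a constant, frame-rate-independent speed.
; When an actor overlap ends, it destroys itself after a zero-length delay; the Getchar function is an empty stub.
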(event `self.ReceiveBeginPlay`)

(event `self.ReceiveTick`
  (params (DeltaSeconds :type "Float (single-precision)"))
  (`SceneComponent.K2_AddLocalOffset` (`self.Cube`) (`KismetMathLibrary.MakeVector` (* (* (`GameplayStatics.GetWorldDeltaSeconds`) 250.0) -1.0)) false false))

(event `self.ReceiveActorEndOverlap`
  (params (OtherActor :type "Actor Object Reference"))
  (`KismetSystemLibrary.Delay` 0.0)
  (`self.K2_DestroyActor`))

(fn `get-char`
  (returns (`char-output` :type "Array of /Game/char-select/char-select Object Reference"))
  (return))

(fn `UserConstructionScript`
  (bind _returnvalue (`PrimitiveComponent.CreateDynamicMaterialInstance` (`self.Cube`) 0 null "None"))
  (`MaterialInstanceDynamic.SetVectorParameterValue` _returnvalue "Color" (`self.NoteColor`)))