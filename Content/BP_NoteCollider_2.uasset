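; Second note hit zone for what appears to be a rhythm game, tracking overlapping notes and scoring their alignment.
; While overlapped, Tick writes the X-axis distance to the game instance, and GetPointsForNote converts it to points.
; End overlap clears Notecollide1 (not Notecollide2) and resets Distance before grading it, so Goodjob feedback always spawns at a jittered position and Early/Late never do.
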(event `self.Collider.OnComponentBeginOverlap`
  (params (OverlappedComponent :type "PrimitiveComponent Object Reference") (OtherActor :type "Actor Object Reference") (OtherComp :type "PrimitiveComponent Object Reference") (OtherBodyIndex :type Integer) (bFromSweep :type Boolean) (SweepResult :type "HitResult Structure (by ref)"))
  (set `self.IsNoteHitting` true)
  (set `self.StartTime` (`KismetSystemLibrary.GetGameTimeInSeconds`)))

(event `self.ReceiveTick`
  (params (DeltaSeconds :type "Float (single-precision)"))
  (if (`self.IsNoteHitting`)
    (bind _returnvalue_x (`KismetMathLibrary.BreakVector` (`SceneComponent.K2_GetComponentLocation` (stale `self.Collider.OnComponentBeginOverlap` OtherComp))))
    (set `self.Distance` (`KismetMathLibrary.Abs` (- (.x (.location (`self.GetTransform`))) _returnvalue_x)))
    (bind _asdata__game_instance (cast `/Game/char-select/Data-Game-instance` (`GameplayStatics.GetGameInstance`)))
    (set `/Game/char-select/Data-Game-instance.note-collide-2` true _asdata__game_instance)
    (set `/Game/char-select/Data-Game-instance.Distance-global-2` (`self.Distance`) _asdata__game_instance)))

(event `self.Collider.OnComponentEndOverlap`
  (params (OverlappedComponent :type "PrimitiveComponent Object Reference") (OtherActor :type "Actor Object Reference") (OtherComp :type "PrimitiveComponent Object Reference") (OtherBodyIndex :type Integer))
  (bind (_returnvalue_x _returnvalue_y _returnvalue_z) (`KismetMathLibrary.BreakVector` (`SceneComponent.K2_GetComponentLocation` OtherComp)))
  (bind (_returnvalue_x_2 _returnvalue_y_2 _returnvalue_z_2) (`KismetMathLibrary.BreakVector` (`SceneComponent.K2_GetComponentLocation` OtherComp)))
  (bind (_returnvalue_x_3 _returnvalue_y_3 _returnvalue_z_3) (`KismetMathLibrary.BreakVector` (`SceneComponent.K2_GetComponentLocation` OtherComp)))
  (set `self.IsNoteHitting` false)
  (set `self.Distance` -1.0)
  (bind _asdata__game_instance (cast `/Game/char-select/Data-Game-instance` (`GameplayStatics.GetGameInstance`)))
  (set `/Game/char-select/Data-Game-instance.note-collide-1` false _asdata__game_instance)
  (if (`KismetMathLibrary.InRange_FloatFloat` (`self.Distance`) -1000.0 1000.0)
    (`|SpawnActorFromClass` "/Game/Layout-assets/Fonts/good-job.good-job_C" (`KismetMathLibrary.MakeTransform` (`KismetMathLibrary.MakeVector` (+ _returnvalue_x -30.0) (+ _returnvalue_y (`KismetMathLibrary.RandomFloatInRange` -20.0 20.0)) (+ _returnvalue_z (`KismetMathLibrary.RandomFloatInRange` -20.0 20.0)))) "Undefined" "MultiplyWithRoot" null null)
    (elif (`KismetMathLibrary.InRange_FloatFloat` (`self.Distance`))
      (`|SpawnActorFromClass` "/Game/Layout-assets/Fonts/early.early_C" (`KismetMathLibrary.MakeTransform` (`KismetMathLibrary.MakeVector` (+ _returnvalue_x_2 -30.0) (+ _returnvalue_y_2 (`KismetMathLibrary.RandomFloatInRange` -20.0 20.0)) (+ _returnvalue_z_2 (`KismetMathLibrary.RandomFloatInRange` -20.0 20.0)))) "Undefined" "MultiplyWithRoot" null null)
      (elif (`KismetMathLibrary.InRange_FloatFloat` (`self.Distance`))
        (`|SpawnActorFromClass` "/Game/Layout-assets/Fonts/late.late_C" (`KismetMathLibrary.MakeTransform` (`KismetMathLibrary.MakeVector` (+ _returnvalue_x_3 -30.0) (+ _returnvalue_y_3 (`KismetMathLibrary.RandomFloatInRange` -20.0 20.0)) (+ _returnvalue_z_3 (`KismetMathLibrary.RandomFloatInRange` -20.0 20.0)))) "Undefined" "MultiplyWithRoot" null null)))))

(fn `get-char`
  (returns (`char-output` :type "Array of /Game/char-select/char-select Object Reference"))
  (return))

(fn `GetPointsForNote`
  (returns (Points :type Integer))
  (if (`self.IsNoteHitting`)
    (return (`KismetMathLibrary.FTrunc` (`KismetMathLibrary.FMax` (+ (* (`self.Distance`) -1.0) 10.0))))
    (else
      (return -1))))

(fn `UserConstructionScript`)