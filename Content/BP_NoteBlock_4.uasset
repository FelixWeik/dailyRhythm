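; BP_NoteBlock_4 is a note block, apparently for a rhythm game, tinted by NoteColor through a dynamic material in construction.
; Its cube slides along local negative X at a constant, frame-rate-independent speed.
; Beginning an overlap sets a flag that lets the Hit-note event destroy the block.
; Ending an overlap adds a mistake to the game instance and destroys the block; Getchar is an empty stub.
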(event `self.ReceiveTick`
  (params (DeltaSeconds :type "Float (single-precision)"))
  ; Move noteblock
  (`SceneComponent.K2_AddLocalOffset` (`self.Cube`) (`KismetMathLibrary.MakeVector` (* (* (`GameplayStatics.GetWorldDeltaSeconds`) 250.0) -1.0)) false false))

(event `self.ReceiveActorEndOverlap`
  (params (OtherActor :type "Actor Object Reference"))
  ; Destroy noteblock
  (bind _asdata__game_instance (cast `/Game/char-select/Data-Game-instance` (`GameplayStatics.GetGameInstance`)))
  (set `/Game/char-select/Data-Game-instance.game-mistakes` (+ (`/Game/char-select/Data-Game-instance.game-mistakes` _asdata__game_instance) 1) _asdata__game_instance)
  (`KismetSystemLibrary.Delay` 0.0)
  (`self.K2_DestroyActor`))

(event `self.ReceiveActorBeginOverlap`
  (params (OtherActor :type "Actor Object Reference"))
  (set `self.overlap` true))

(event `/Game/char-select/Interface-char-select.hit-note`
  (if (`self.overlap`)
    (`self.K2_DestroyActor`)))

(fn `get-char`
  (returns (`char-output` :type "Array of /Game/char-select/char-select Object Reference"))
  (return))

(fn `UserConstructionScript`
  (bind _returnvalue (`PrimitiveComponent.CreateDynamicMaterialInstance` (`self.Cube`) 0 null "None"))
  (`MaterialInstanceDynamic.SetVectorParameterValue` _returnvalue "Color" (`self.NoteColor`)))