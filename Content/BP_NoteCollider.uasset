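; BP_NoteCollider is a note hit-detection actor that measures how closely an overlapping component aligns with it and scores that timing.
; Collider overlap events toggle IsNoteHitting; while it is set, Tick computes and prints the Y-axis distance to the component.
; Tick publishes that distance and a collide flag to the Data-Game-instance, and end overlap clears the flag.
; GetPointsForNote returns higher points for smaller distances, or -1 without an overlap.
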(event `self.ReceiveBeginPlay`)

(event `self.ReceiveTick`
  (params (DeltaSeconds :type "Float (single-precision)"))
  (if (`self.IsNoteHitting`)
    (bind (_returnvalue_x _returnvalue_y) (`KismetMathLibrary.BreakVector` (`SceneComponent.K2_GetComponentLocation` (stale `self.Collider.OnComponentBeginOverlap` OtherComp))))
    (bind _output_get (set `self.Distance` (`KismetMathLibrary.Abs` (- (.y (.location (`self.GetTransform`))) _returnvalue_y))))
    (`KismetSystemLibrary.PrintString` (`KismetStringLibrary.Conv_DoubleToString` _output_get))
    (bind _asdata__game_instance (cast `/Game/char-select/Data-Game-instance` (`GameplayStatics.GetGameInstance`)))
    (set `/Game/char-select/Data-Game-instance.note-collide` true _asdata__game_instance)
    (set `/Game/char-select/Data-Game-instance.Distance-global` (`self.Distance`) _asdata__game_instance)))

(event `self.Collider.OnComponentEndOverlap`
  (params (OverlappedComponent :type "PrimitiveComponent Object Reference") (OtherActor :type "Actor Object Reference") (OtherComp :type "PrimitiveComponent Object Reference") (OtherBodyIndex :type Integer))
  (set `self.IsNoteHitting` false)
  (set `self.Distance` -1.0)
  (bind _asdata__game_instance (cast `/Game/char-select/Data-Game-instance` (`GameplayStatics.GetGameInstance`)))
  (set `/Game/char-select/Data-Game-instance.note-collide` false _asdata__game_instance))

(event `self.Collider.OnComponentBeginOverlap`
  (params (OverlappedComponent :type "PrimitiveComponent Object Reference") (OtherActor :type "Actor Object Reference") (OtherComp :type "PrimitiveComponent Object Reference") (OtherBodyIndex :type Integer) (bFromSweep :type Boolean) (SweepResult :type "HitResult Structure (by ref)"))
  (set `self.IsNoteHitting` true)
  (set `self.StartTime` (`KismetSystemLibrary.GetGameTimeInSeconds`)))

(fn `get-char`
  (returns (`char-output` :type "Array of /Game/char-select/char-select Object Reference"))
  (return))

(fn `GetPointsForNote`
  (returns (Points :type Integer))
  (if (`self.IsNoteHitting`)
    (return (`KismetMathLibrary.FTrunc` (`KismetMathLibrary.FMax` (+ (* (`self.Distance`) -1.0) 10.0))))
    (else
      (return -1))))

(fn `UserConstructionScript`)